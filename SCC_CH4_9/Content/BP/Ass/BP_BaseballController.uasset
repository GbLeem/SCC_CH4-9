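; Player controller for a turn-based number baseball guessing game between host and guest, played through chat messages.
; On BeginPlay it binds to the WBP_Chat widget, and its send event forwards message text with the user ID to BP_BaseballGameMode.
; On broadcasts, the authority asks the game mode to check for a win, then prints a win, tie or next turn.
; A win or exhausted guest count resets turns and generates a new number.
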(event Custom|OnSendMessageToServer
  (params (Message :type String))
  (bind _asbp_baseball_game_mode (Utilities|Casting|CastToBP_BaseballGameMode (Game|GetGameMode)))
  (Default|GotMessagefromClient _asbp_baseball_game_mode (.RightS (Utilities|String|Split Message "/")) (Variables|Default|GetUserID)))

(event Custom|OnLogInWithID
  (params (UserID :type String))
  (Variables|Default|SetUserID UserID))

(event Custom|Got%20Broadcast
  (params (Message :type String))
  (if (Ability|HasAuthority)
    (Development|PrintString Message true true "(R=0.000000,G=0.660000,B=1.000000,A=1.000000)" 1e+01)
    (bind _asbp_baseball_game_mode (Utilities|Casting|CastToBP_BaseballGameMode (Game|GetGameMode)))
    ;[0.15 0.15 0.15 0.5] game win
    (bind _returnvalue (Class|BaseBallGameMode|WinCheck _asbp_baseball_game_mode (.RightS (Utilities|String|Split Message "result : "))))
    (if _returnvalue
      (Development|PrintString (Utilities|String|Append (Variables|Default|GetUserID) " WIN!") true true "(R=0.000000,G=0.660000,B=1.000000,A=1.000000)" 1e+01)
      (Development|PrintString "===RESET===" true true "(R=0.000000,G=0.660000,B=1.000000,A=1.000000)" 1e+01)
      (Class|BaseBallGameMode|ResetTurnandCount _asbp_baseball_game_mode)
      (Class|BaseBallGameMode|MakeRandomNumber _asbp_baseball_game_mode)
      (elif (> (Variables|/Script/SCC_CH4_9.BaseBallGameMode|GetGuestCount _asbp_baseball_game_mode) 0)
        (if (== (Math|Integer|%(Integer) (Variables|/Script/SCC_CH4_9.BaseBallGameMode|GetTurnIndex _asbp_baseball_game_mode) 2) 0)
          (Development|PrintString "GUEST TURN" true true "(R=1.000000,G=0.000000,B=0.000000,A=1.000000)" 1e+01)
          (else
            (Development|PrintString "HOST TURN" true true "(R=1.000000,G=0.000000,B=0.000000,A=1.000000)" 1e+01)))
        (else
          ;[0.15 0.15 0.15 0.5] game tie
          (Development|PrintString "TIE GAME" true true "(R=0.000000,G=0.660000,B=1.000000,A=1.000000)" 1e+01)
          (Development|PrintString "===RESET===" true true "(R=0.000000,G=0.660000,B=1.000000,A=1.000000)" 1e+01)
          (Class|BaseBallGameMode|ResetTurnandCount _asbp_baseball_game_mode)
          (Class|BaseBallGameMode|MakeRandomNumber _asbp_baseball_game_mode))))))

(event EventBeginPlay
  (CallFunction|ResetGame))

(fn ConstructionScript)

(fn ResetGame
  (if (not (Utilities|Enum|Equal(Enum) (Class|Actor|GetRemoteRole) "ROLE_None"))
    (bind _foundwidgets (Widget|GetAllWidgetsOfClass "/Game/BP/Ass/WBP_Chat.WBP_Chat_C" true))
    (EventDispatchers|BindEventtoSetMessagetoUserController (Utilities|Array|Get(acopy) _foundwidgets) (EventDispatchers|CreateEvent :!event Custom|OnSendMessageToServer))))

(fn CheckTurn
  (bind _asbp_baseball_game_mode (Utilities|Casting|CastToBP_BaseballGameMode (Game|GetGameMode)))
  (return (== (Math|Integer|%(Integer) (Variables|/Script/SCC_CH4_9.BaseBallGameMode|GetTurnIndex _asbp_baseball_game_mode) 2) 0)))