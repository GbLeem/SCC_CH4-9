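; Game mode for a turn-based Host vs Guest baseball number game played through client messages.
; On BeginPlay it makes a random number and resets the turn and chance counts.
; Each client message is checked for turn and sender, scored with GetResult, then broadcast to every BP_BaseballController with that player's remaining chances.
; ShowTurnUI, re-fired inside that broadcast loop, labels the turn on all controllers from TurnIndex parity.
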(event Custom|GotMessageFromClient
  (params (Message :type String) (UserID :type String))
  (bind _returnvalue (Class|BaseBallGameMode|CheckTurnandID UserID))
  (if (or (== _returnvalue 1) (== _returnvalue 2))
    (bind _returnvalue_2 (Class|BaseBallGameMode|GetResult Message))
    (bind _outactors (Actor|GetAllActorsOfClass "/Script/Engine.PlayerController"))
    (for _array_element _outactors
      (bind _asbp_baseball_controller (Utilities|Casting|CastToBP_BaseballController _array_element))
      (Utilities|FlowControl|Sequence
        (:then_0
          (if (== _returnvalue 1)
            (Default|GotBroadcast _asbp_baseball_controller (Utilities|String|Append UserID " | remain chance : " (Utilities|String|ToString(Integer) (Variables|Default|GetHostCount)) " | result : " _returnvalue_2))
            (CallFunction|ShowTurnUI :!label _label)))
        (:then_1
          (if (== _returnvalue 2)
            (Default|GotBroadcast _asbp_baseball_controller (Utilities|String|Append UserID " | remain chance : " (Utilities|String|ToString(Integer) (Variables|Default|GetGuestCount)) " | result : " _returnvalue_2))
            (goto _label)))))))

(event Custom|ShowTurnUI
  (bind _outactors (Actor|GetAllActorsOfClass "/Game/BP/Ass/BP_BaseballController.BP_BaseballController_C"))
  (for _array_element _outactors
    (if (== (Math|Integer|%(Integer) (Variables|Default|GetTurnIndex) 2) 0)
      (Default|ShowTurnUI _array_element "GUEST TURN")
      (else
        (Default|ShowTurnUI _array_element "HOST TURN")))))

(event EventBeginPlay
  (Class|BaseBallGameMode|MakeRandomNumber)
  (Class|BaseBallGameMode|ResetTurnandCount)
  (Development|PrintString "HOST Turn" true true "(R=1.000000,G=0.000000,B=0.011301,A=1.000000)" 1e+01))

(fn ConstructionScript)