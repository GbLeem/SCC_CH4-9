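; Player controller for a chat game, linking the WBP_Chat widget to BP_ChatGameMode.
; On BeginPlay, when a remote role exists, it waits briefly, then binds an event to the first chat widget found.
; Outgoing messages get the stored login UserId prefixed and go to the game mode's GotMessageFromClient.
; Received broadcasts are printed on screen only with authority; a CallOnUserLogIn call is left unconnected.
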(event Custom|OnSendMsgToServer
  (params (Message :type String))
  (bind _asbp_chat_game_mode (Utilities|Casting|CastToBP_ChatGameMode (Game|GetGameMode)))
  (Default|GotMessagefromClient _asbp_chat_game_mode (Utilities|String|Append (Variables|Default|GetUserId) ": " Message)))

(event Custom|GotBroadCast
  (params (Message :type String))
  (if (Ability|HasAuthority)
    (Development|PrintString Message true true "(R=0.000000,G=0.660000,B=1.000000,A=1.000000)" 1e+01)))

(event Custom|OnLogInWithID
  (params (UserId :type String))
  (Variables|Default|SetUserId UserId))

(event EventBeginPlay
  (if (not (Utilities|Enum|Equal(Enum) (Class|Actor|GetRemoteRole) "ROLE_None"))
    (Utilities|FlowControl|Delay 0.2)
    (bind _foundwidgets (Widget|GetAllWidgetsOfClass "/Game/BP/WBP_Chat.WBP_Chat_C" true))
    (bind _output_get (Variables|Default|SetWidget (Utilities|Array|Get(acopy) _foundwidgets)))
    (EventDispatchers|BindEventtoSetMessagetoUserController _output_get (EventDispatchers|CreateEvent :!event Custom|OnSendMsgToServer))))

(fn ConstructionScript)